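; Recruit playable character Blueprint with two skills, sprint and grenade, built as components on a parent character class.
; BeginPlay initializes health, armor and shield, then initializes both skill components and registers them in the Skills array.
; Skill_0 input fires and finishes sprint, disabling grenade meanwhile, while Skill_1 fires the grenade from its spawn point.
; Tick disables sprint while the grenade is in one particular state, making the skills mutually exclusive.
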(event Input|EnhancedActionEvents|EnhancedInputActionSkill_0
  (params (ActionValue :type Boolean) (ElapsedSeconds :type Float%20%28double-precision%29) (TriggeredSeconds :type Float%20%28double-precision%29) (InputAction :type Input%20Action%20Object%20Reference :default "/Game/_Project/Input/Skill_0.Skill_0"))
  (bind _recruit_sprint_skill_bpc (Variables|Default|GetRecruit_Sprint_Skill_BPC))
  (bind _recruit_grenade_skill_bpc (Variables|Default|GetRecruit_Grenade_Skill_BPC))
  (:Triggered
    (Default|Fire _recruit_sprint_skill_bpc :!label _label)
    (Default|SetEnabled _recruit_grenade_skill_bpc false))
  (:Started
    (goto _label))
  (:Canceled
    (Default|Finish _recruit_sprint_skill_bpc :!label _label_2)
    (Default|SetEnabled _recruit_grenade_skill_bpc true))
  (:Completed
    (goto _label_2)))

(event Input|EnhancedActionEvents|EnhancedInputActionSkill_1
  (params (ActionValue :type Boolean) (ElapsedSeconds :type Float%20%28double-precision%29) (TriggeredSeconds :type Float%20%28double-precision%29) (InputAction :type Input%20Action%20Object%20Reference :default "/Game/_Project/Input/Skill_1.Skill_1"))
  (bind _recruit_grenade_skill_bpc (Variables|Default|GetRecruit_Grenade_Skill_BPC))
  (:Started
    (Variables|/Game/_Project/Characters/Recruit/Skills/Grenade/Recruit_Grenade_Skill_BPC.Recruit_Grenade_Skill_BPC_C|SetSpawnPoint _recruit_grenade_skill_bpc (Transformation|GetWorldTransform (Variables|Default|GetGrenadeSpawnPoint)))
    (Default|Fire _recruit_grenade_skill_bpc)))

(event EventBeginPlay
  (bind _recruit_sprint_skill_bpc (Variables|Default|GetRecruit_Sprint_Skill_BPC))
  (bind _recruit_grenade_skill_bpc (Variables|Default|GetRecruit_Grenade_Skill_BPC))
  (|CallParentFunction)
  (Utilities|FlowControl|Sequence
    (:then_0
      (CallFunction|InitializeHealth (Utilities|Struct|MakeHealthData 125.0 125.0 5e+01 5e+01 5e+01 5e+01 0.0 false)))
    (:then_1
      (Default|Initialize _recruit_grenade_skill_bpc self)
      (Utilities|Array|Add (Variables|Default|GetSkills) _recruit_grenade_skill_bpc))
    (:then_2
      (Default|Initialize _recruit_sprint_skill_bpc self)
      (Utilities|Array|Add (Variables|Default|GetSkills) _recruit_sprint_skill_bpc))))

(event EventTick
  (params (DeltaSeconds :type Float%20%28single-precision%29))
  (|CallParentFunction DeltaSeconds)
  (Default|SetEnabled (Variables|Default|GetRecruit_Sprint_Skill_BPC) (Utilities|Enum|NotEqual(Enum) (Variables|/Game/_Project/CommonSystems/Character_Skills/Character_Skill_BP.Character_Skill_BP_C|GetState (Variables|Default|GetRecruit_Grenade_Skill_BPC)) "NewEnumerator1")))

(fn ConstructionScript
  (|CallParentFunction))
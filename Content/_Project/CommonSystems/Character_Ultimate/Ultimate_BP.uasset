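; Ultimate Blueprint that tracks the charge of a character's ultimate ability.
; Initialize stores the owning character, registers the ultimate UI through that character's UI, zeroes the display and starts a looping one-second timer.
; While in its first state, each tick adds the charge rate, clamps on overflow past the maximum and switches to the second state.
; The UI receives current charge modulo maximum rather than a ratio.
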(event Custom|Initialize
  (params (OwningCharacter :type Base%20Character%20BP%20Object%20Reference))
  (bind _ultimateui (Variables|Default|GetUltimateUI))
  (Utilities|FlowControl|Sequence
    (:then_0
      (Variables|Default|SetOwningCharacter OwningCharacter))
    (:then_1
      (Default|SetUltimateUI (Variables|/Game/_Project/Characters/BaseCharacter_BP.BaseCharacter_BP_C|GetUI (Variables|Default|GetOwningCharacter)) _ultimateui)
      (Default|SetUltimatePercentage _ultimateui 0.0))
    (:then_2
      (Utilities|Time|SetTimerbyEvent (delegate Custom|UpdateUltimateCharge) 1.0 true))))

(event Custom|UpdateUltimateCharge
  (if (Utilities|Enum|Equal(Enum) (Variables|Default|GetState) "NewEnumerator0")
    (if (> (+ (Variables|Default|GetCurrentCharge) (Variables|Default|GetChargeRate)) (Variables|Default|GetMaxCharge))
      (Variables|Default|SetCurrentCharge (Variables|Default|GetMaxCharge))
      (Variables|Default|SetState "NewEnumerator1")
      (else
        (Variables|Default|SetCurrentCharge (+ (Variables|Default|GetCurrentCharge) (Variables|Default|GetChargeRate)))))
    (Default|SetUltimatePercentage (Variables|Default|GetUltimateUI) (Math|Float|%(Float) (Variables|Default|GetCurrentCharge) (Variables|Default|GetMaxCharge)))))
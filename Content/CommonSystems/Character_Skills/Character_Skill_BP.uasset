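; Base character skill Blueprint that holds a skill's owning character, enabled flag and state machine, with an empty Update for per-frame logic.
; Fire moves an enabled skill from its initial state to a second state, and Finish moves it to a third until a FinishTime timer resets it.
; Enabling sets the second state unless a fourth is current, while disabling cancels the timer without changing state.
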(event Custom|SetEnabled
  (params (Enabled? :type Boolean))
  (bind _output_get (Variables|Default|SetEnabled Enabled?))
  (if _output_get
    (if (Utilities|Enum|NotEqual(Enum) (Variables|Default|GetState) "NewEnumerator3")
      (Variables|Default|SetState "NewEnumerator1"))
    (else
      (Utilities|Time|ClearandInvalidateTimerbyHandle (Variables|Default|GetFinishTimerHandle)))))

(event Custom|Initialize
  (params (OwningCharacter :type Base%20Character%20BP%20Object%20Reference))
  (Utilities|FlowControl|Sequence
    (:then_0
      (Variables|Default|SetState "NewEnumerator0"))
    (:then_1
      (Variables|Default|SetOwningCharacter OwningCharacter))))

(event Custom|OnFinish
  (Variables|Default|SetState "NewEnumerator0"))

(event Custom|Fire
  (if (and (Utilities|Enum|Equal(Enum) (Variables|Default|GetState) "NewEnumerator0") (Variables|Default|GetEnabled))
    (Variables|Default|SetState "NewEnumerator1")))

(event Custom|Update
  (params (DeltaTime :type Float%20%28double-precision%29)))

(event Custom|Finish
  (if (Utilities|Enum|Equal(Enum) (Variables|Default|GetState) "NewEnumerator1")
    (Variables|Default|SetState "NewEnumerator2")
    (bind _returnvalue (Utilities|Time|SetTimerbyEvent (delegate Custom|OnFinish) (Variables|Default|GetFinishTime)))
    (Variables|Default|SetFinishTimerHandle _returnvalue)))
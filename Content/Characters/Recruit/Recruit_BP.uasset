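; Recruit is a playable character Blueprint that extends a parent character with its own health pool and a sprint skill.
; On BeginPlay it initializes health, armor and shield, then initializes the sprint skill component and registers it in the Skills array.
; The Skill_0 input action fires the sprint on Started and Triggered, and finishes it on Completed or Canceled.
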(event Input|EnhancedActionEvents|EnhancedInputActionSkill_0
  (params (ActionValue :type Boolean) (ElapsedSeconds :type Float%20%28double-precision%29) (TriggeredSeconds :type Float%20%28double-precision%29) (InputAction :type Input%20Action%20Object%20Reference :default "/Game/Input/Skill_0.Skill_0"))
  (bind _recruit_sprint_skill_bpc (Variables|Default|GetRecruit_Sprint_Skill_BPC))
  (:Triggered
    (Default|Fire _recruit_sprint_skill_bpc :!label _label))
  (:Started
    (goto _label))
  (:Canceled
    (Default|Finish _recruit_sprint_skill_bpc :!label _label_2))
  (:Completed
    (goto _label_2)))

(event EventBeginPlay
  (bind _recruit_sprint_skill_bpc (Variables|Default|GetRecruit_Sprint_Skill_BPC))
  (|CallParentFunction)
  (Utilities|FlowControl|Sequence
    (:then_0
      (CallFunction|InitializeHealth (Utilities|Struct|MakeHealthData 125.0 125.0 5e+01 5e+01 5e+01 5e+01 0.0 false)))
    (:then_1
      (Default|Initialize _recruit_sprint_skill_bpc self)
      (Utilities|Array|Add (Variables|Default|GetSkills) _recruit_sprint_skill_bpc))))

(fn ConstructionScript
  (|CallParentFunction))
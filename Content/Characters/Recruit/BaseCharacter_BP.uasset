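; Recruit base character Blueprint: a first-person playable character with a weapon, layered health and a charging ultimate.
; BeginPlay adds Enhanced Input mapping, creates the HUD, and initializes the weapon (camera as fire point) and health system (health, armor, shield).
; Tick updates health, HUD bar and weapon, while a looping timer fills ultimate charge until ready.
; Input drives movement, look and jump, and forwards fire and reload to the weapon.
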(event Custom|UpdateHealthUI
  (Default|SetHealthBar (Variables|Default|GetUI) (Default|GetHealthData (Variables|Default|GetHealthSystem))))

(event Custom|UpdateUltimateCharge
  (if (not (Variables|Ultimate|GetUltimateReady))
    (if (> (+ (Variables|Ultimate|GetCurrentUltimateCharge) (Variables|Ultimate|GetUltimateChargeRate)) (Variables|Ultimate|GetMaxUltimateCharge))
      (Variables|Ultimate|SetCurrentUltimateCharge (Variables|Ultimate|GetMaxUltimateCharge))
      (Variables|Ultimate|SetUltimateReady true)
      (else
        (Variables|Ultimate|SetCurrentUltimateCharge (+ (Variables|Ultimate|GetCurrentUltimateCharge) (Variables|Ultimate|GetUltimateChargeRate)))))
    (Default|SetUltimatePercentage (Variables|Default|GetUI) (/ (Variables|Ultimate|GetCurrentUltimateCharge) (Variables|Ultimate|GetMaxUltimateCharge)))))

(event Input|EnhancedActionEvents|EnhancedInputActionJump
  (params (ActionValue :type Boolean) (ElapsedSeconds :type Float%20%28double-precision%29) (TriggeredSeconds :type Float%20%28double-precision%29) (InputAction :type Input%20Action%20Object%20Reference :default "/Game/Input/Jump.Jump"))
  (:Started
    (Character|Jump))
  (:Canceled
    (Character|StopJumping :!label _label))
  (:Completed
    (goto _label)))

(event Input|EnhancedActionEvents|EnhancedInputActionLook
  (params (ActionValue :type Vector%202D%20Structure) (ElapsedSeconds :type Float%20%28double-precision%29) (TriggeredSeconds :type Float%20%28double-precision%29) (InputAction :type Input%20Action%20Object%20Reference :default "/Game/Input/Look.Look"))
  (bind (_x _y) (Math|Vector2D|BreakVector2D ActionValue))
  (Pawn|Input|AddControllerYawInput _x)
  (Pawn|Input|AddControllerPitchInput _y))

(event Input|EnhancedActionEvents|EnhancedInputActionMove
  (params (ActionValue :type Vector%202D%20Structure) (ElapsedSeconds :type Float%20%28double-precision%29) (TriggeredSeconds :type Float%20%28double-precision%29) (InputAction :type Input%20Action%20Object%20Reference :default "/Game/Input/Move.Move"))
  (bind (_x _y) (Math|Vector2D|BreakVector2D ActionValue))
  (Pawn|Input|AddMovementInput (Math|Vector|GetForwardVector (Variables|Collision|GetCapsuleComponent)) _x false)
  (Pawn|Input|AddMovementInput (Math|Vector|GetRightVector (Variables|Collision|GetCapsuleComponent)) _y false))

(event Input|EnhancedActionEvents|EnhancedInputActionPrimaryFire
  (params (ActionValue :type Boolean) (ElapsedSeconds :type Float%20%28double-precision%29) (TriggeredSeconds :type Float%20%28double-precision%29) (InputAction :type Input%20Action%20Object%20Reference :default "/Game/Input/PrimaryFire.PrimaryFire"))
  (bind _recruit_weapon (Variables|Default|GetRecruit_Weapon))
  (:Started
    (Default|StartFireWeapon _recruit_weapon))
  (:Canceled
    (Default|StopFireWeapon _recruit_weapon :!label _label))
  (:Completed
    (goto _label)))

(event Input|EnhancedActionEvents|EnhancedInputActionReload
  (params (ActionValue :type Boolean) (ElapsedSeconds :type Float%20%28double-precision%29) (TriggeredSeconds :type Float%20%28double-precision%29) (InputAction :type Input%20Action%20Object%20Reference :default "/Game/Input/Reload.Reload"))
  (:Started
    (Default|Reload (Variables|Default|GetRecruit_Weapon))))

(event EventBeginPlay
  (Utilities|FlowControl|Sequence
    (:then_0
      (CallFunction|SetInputMappingContext "/Game/Input/BaseCharacterMapping.BaseCharacterMapping"))
    (:then_1
      (CallFunction|CreateCharacterUI "/Game/UI/BaseUI/BaseCharacter_UI.BaseCharacter_UI_C")
      (bind _output_get (Variables|Default|SetAnimation (.AsRecruit%20Animation%20BP (Utilities|Casting|CastToRecruit_AnimationBP (Components|SkeletalMesh|GetAnimInstance (Variables|Character|GetMesh))))))
      (Default|Initialize (Variables|Default|GetRecruit_Weapon) _output_get (Variables|Default|GetCamera) (Variables|/Game/UI/BaseUI/BaseCharacter_UI.BaseCharacter_UI_C|GetWeapon_UI (Variables|Default|GetUI))))
    (:then_2
      (Default|Initialize (Variables|Default|GetHealthSystem) (Utilities|Struct|MakeHealthData 2e+02 2e+02 1.5e+02 1.5e+02 5e+01 5e+01 0.0 false))
      (CallFunction|UpdateHealthUI))
    (:then_3
      (Utilities|Time|SetTimerbyEvent (delegate Custom|UpdateUltimateCharge) 1.0 true))))

(event EventTick
  (params (DeltaSeconds :type Float%20%28single-precision%29))
  (Default|Update (Variables|Default|GetHealthSystem) DeltaSeconds)
  (CallFunction|UpdateHealthUI)
  (Default|Update (Variables|Default|GetRecruit_Weapon)))

(fn ConstructionScript)

(fn SetInputMappingContext
  (params (MappingContext :type Input%20Mapping%20Context%20Object%20Reference))
  (Input|AddMappingContext (PlayerController|LocalPlayerSubsystems|GetEnhancedInputLocalPlayerSubsystem (Game|GetPlayerController 0)) MappingContext 0 "(bIgnoreAllPressedKeysUntilRelease=True,bForceImmediately=False,bNotifyUserSettings=False)"))

(fn CreateCharacterUI
  (params (UI%20Class :type Base%20Character%20UI%20Class%20Reference))
  (bind _returnvalue (UserInterface|CreateWidget UI%20Class (Game|GetPlayerController 0)))
  (bind _output_get (Variables|Default|SetUI _returnvalue))
  (UserInterface|Viewport|AddtoViewport _output_get 0)
  (Default|SetCharacterName _output_get (Variables|Default|GetName))
  (Default|SetUltimatePercentage _output_get 0.0))